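; Statue fire prop that turns blue when the game's lap counter reaches 3.
; BeginPlay caches the Global_Variables game instance.
; Tick polls CurrentLapCounter and, while it equals 3, swaps the Niagara fire effect to NS_Fire_Blue and tints the point light blue.
; The swap has no one-shot guard, so it is reapplied every frame during that lap, and nothing reverts it.
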(event `self.ReceiveBeginPlay`
  (bind _asglobal_variables (cast `Global_Variables` (`GameplayStatics.GetGameInstance`)))
  (set `self.AsGlobal Variables` _asglobal_variables))

(event `self.ReceiveTick`
  (params (DeltaSeconds :type "Float (single-precision)"))
  (if (== 3 (`Global_Variables.CurrentLap_Counter` (`self.AsGlobal Variables`)))
    (`NiagaraComponent.SetAsset` (`self.FireEffect`) "/Game/Misc/Niagara/NS_Fire_Blue.NS_Fire_Blue" true)
    (`LightComponent.SetLightColor` (`self.PointLight`) (struct :`R` 0.133779 :`G` 0.484565 :`B` 0.751042 :`A` 1.0) true)))

(fn `UserConstructionScript`)