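; Player controller that lets a gamepad's left stick move the mouse cursor.
; Both left-stick axis events share one branch, gated by ShouldUseGamepadInput, that offsets the current mouse position by scaled axis input, with the vertical offset negated.
; The result is truncated to integers and clamped to the viewport bounds before the cursor location is set.
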(event `InputAxisKey|Gamepad_LeftX` :paused true
  (params (AxisValue :type "Float (single-precision)"))
  (bind (_sizex _sizey) (`self.GetViewportSize`))
  (bind (_locationx _locationy) (`self.GetMousePosition`))
  ;[0 0 0] Handle gamepad mouse cursor input
  (if (`self.ShouldUseGamepadInput`) :!label _label
    (`self.SetMouseLocation` (`KismetMathLibrary.Clamp` (`KismetMathLibrary.FTrunc` (+ (* AxisValue 5.0) _locationx)) 0 _sizex) (`KismetMathLibrary.Clamp` (`KismetMathLibrary.FTrunc` (+ (* (stale `InputAxisKey|Gamepad_LeftY` AxisValue) -5.0) _locationy)) 0 _sizey))))

(event `InputAxisKey|Gamepad_LeftY` :paused true
  (params (AxisValue :type "Float (single-precision)"))
  ;[0 0 0] Handle gamepad mouse cursor input
  (goto _label))

(event `Key|Gamepad_FaceButton_Bottom`
  (params (Key :type "Key Structure")))

(fn `UserConstructionScript`)