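; Track spline actor that builds track geometry by laying meshes along its Spline in the construction script.
; Each TrackSplineStruct entry supplies a mesh, a segment length (Divisor) and a Tangent flag, with segment count derived from spline length.
; Only flagged entries create spline mesh components, bent between sampled local positions using spline direction plus TangentFloat as tangents.
; The event graph is unused.
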(fn `UserConstructionScript`
  (bind _distanceb (`self.DistanceB`))
  (bind _divisor (`self.Divisor`))
  (bind _spline (`self.Spline`))
  (bind _distancea (`self.DistanceA`))
  (for _index (range (+ (`KismetArrayLibrary.Array_Length` (`self.TrackSplineStruct`)) 1))
    (bind (_mesh _divisor_2 _tangent) (break `/Game/Blueprints/Track/TrackSplineStruct` (`|GetArrayItem` (`self.TrackSplineStruct`) _index)))
    (set `self.Mesh` _mesh)
    (set `self.Divisor` _divisor_2)
    (set `self.Tangent` _tangent)
    (for _index_2 (range (+ (`.ReturnValue` (`KismetMathLibrary.FMod` (`SplineComponent.GetSplineLength` (`self.Spline`)) (`self.Divisor`))) 1))
      (bind _returnvalue (* _index_2 _divisor))
      (set `self.DistanceA` _returnvalue)
      (set `self.DistanceB` (+ _returnvalue _divisor))
      (if (`self.Tangent`)
        (bind _returnvalue_2 (`AddComponent|NODE_AddSplineMeshComponent-0`))
        (`StaticMeshComponent.SetStaticMesh` _returnvalue_2 (`self.Mesh`))
        (`SplineMeshComponent.SetStartAndEnd` _returnvalue_2 (`SplineComponent.GetLocationAtDistanceAlongSpline` _spline _distancea "Local") (+ (`SplineComponent.GetDirectionAtDistanceAlongSpline` _spline _distancea "Local") (`self.TangentFloat`)) (`SplineComponent.GetLocationAtDistanceAlongSpline` _spline _distanceb "Local") (+ (`SplineComponent.GetDirectionAtDistanceAlongSpline` _spline _distanceb "Local") (`self.TangentFloat`)) true)))))