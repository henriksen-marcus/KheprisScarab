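; Player ship Blueprint that, in the logic shown, handles only the pause menu.
; BeginPlay creates the pause widget, adds it hidden to the viewport and sets game-only input.
; The Pause action reveals the menu, switches to UI-only input, places the cursor just below screen center and pauses the game.
; An unconnected slow-motion toggle using global time dilation never runs.
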(event `self.ReceiveBeginPlay`
  (bind _returnvalue (`|CreateWidget` "/Game/Blueprints/UI/Menu_Pause_BP.Menu_Pause_BP_C"))
  (`UserWidget.AddToViewport` _returnvalue 0)
  (`Widget.SetVisibility` _returnvalue "Hidden")
  (set `UserWidget.bIsFocusable` true _returnvalue)
  (`WidgetBlueprintLibrary.SetInputMode_GameOnly` (`GameplayStatics.GetPlayerController` 0)))

(event `InputAction|Pause`
  (params (Key :type "Key Structure"))
  (bind _returnvalue (`GameplayStatics.GetPlayerController` 0))
  (bind (_sizex _sizey) (`PlayerController.GetViewportSize` _returnvalue))
  (:`Pressed`
    (`Widget.SetVisibility` (stale `self.ReceiveBeginPlay` _returnvalue) "Visible")
    (`WidgetBlueprintLibrary.SetInputMode_UIOnlyEx` _returnvalue (stale `self.ReceiveBeginPlay` _returnvalue))
    (`PlayerController.SetMouseLocation` _returnvalue (/ _sizex 2) (+ (/ _sizey 2) 100))
    (`GameplayStatics.SetGamePaused` true)))

(event `Key|LeftAlt`
  (params (Key :type "Key Structure")))

(fn `UserConstructionScript`)