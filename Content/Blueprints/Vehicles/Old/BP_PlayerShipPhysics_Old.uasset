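; Older player ship Blueprint that handles the pause menu and a slow-motion toggle, despite its physics name.
; BeginPlay creates a hidden pause widget, which the Pause input reveals before pausing the game; Left Alt toggles global time dilation.
; An unwired CheckUnderlyingSurface function traces downward with debug drawing, attaching a Niagara sand effect over sand physical material and destroying it otherwise.
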(event `self.ReceiveBeginPlay`
  (bind _returnvalue (`|CreateWidget` "/Game/Blueprints/UI/PauseScreen1.PauseScreen1_C"))
  (`UserWidget.AddToViewport` _returnvalue 0)
  (`Widget.SetVisibility` _returnvalue "Hidden")
  (set `UserWidget.bIsFocusable` true _returnvalue))

(event `self.ReceiveTick`
  (params (DeltaSeconds :type "Float (single-precision)")))

(event `InputAction|Pause`
  (params (Key :type "Key Structure"))
  (bind _returnvalue (`GameplayStatics.GetPlayerController` 0))
  (bind (_sizex _sizey) (`PlayerController.GetViewportSize` _returnvalue))
  (:`Pressed`
    (`Widget.SetVisibility` (stale `self.ReceiveBeginPlay` _returnvalue) "Visible")
    (`WidgetBlueprintLibrary.SetInputMode_UIOnlyEx` _returnvalue (stale `self.ReceiveBeginPlay` _returnvalue))
    (`PlayerController.SetMouseLocation` _returnvalue (/ _sizex 2) (+ (/ _sizey 2) 100))
    (`/Game/Blueprints/UI/PauseScreen1.MenuOpened` (stale `self.ReceiveBeginPlay` _returnvalue))
    (`GameplayStatics.SetGamePaused` true)))

(event `Key|LeftAlt`
  (params (Key :type "Key Structure"))
  (:`Pressed`
    (if (== (`GameplayStatics.GetGlobalTimeDilation`) 1.0)
      (`GameplayStatics.SetGlobalTimeDilation` 0.1)
      (else
        (`GameplayStatics.SetGlobalTimeDilation` 1.0)))))

(fn `CheckUnderlyingSurface`
  (bind _returnvalue (`self.K2_GetActorLocation`))
  (bind _sandsystemref (`self.SandSystemRef`))
  (bind (_outhit _returnvalue_2) (`KismetSystemLibrary.LineTraceSingle` _returnvalue (+ _returnvalue (* (`KismetMathLibrary.Vector_Down`) 1000.0)) "TraceTypeQuery1"))
  (bind (_bblockinghit _binitialoverlap _time _distance _location _impactpoint _normal _impactnormal _physmat _hitactor _hitcomponent _hitbonename _hititem _elementindex _faceindex _tracestart _traceend) (`GameplayStatics.BreakHitResult` _outhit))
  (`KismetSystemLibrary.DrawDebugLine` _tracestart _traceend (struct :`R` 1.0 :`A` 1.0) 0.0 12.0)
  (if _returnvalue_2
    (`KismetSystemLibrary.DrawDebugSphere` _impactpoint 50.0 12 (struct :`G` 1.0 :`B` 0.01188 :`A` 1.0) 0.0 6.0)
    (if (== "/Game/Misc/Materials/PM_Sand.PM_Sand" _physmat)
      (`self.SandSys` _location)
      (`VisualLoggerKismetLibrary.LogText` null (`KismetSystemLibrary.GetDisplayName` _physmat) "VisLogBP" true)
      (else
        (`/Engine/EditorBlueprintResources/StandardMacros.IsValid` _sandsystemref :!label _label
          (:`Is Valid`
            (`ActorComponent.K2_DestroyComponent` _sandsystemref)
            (`VisualLoggerKismetLibrary.LogText` null "DestroyedSand!" "VisLogBP" true)))))
    (else
      (goto _label))))

(fn `SandSys`
  (params (HitLocation :type "Vector Structure"))
  (locals (NewLocalVar_0 :type "NiagaraComponent Object Reference"))
  (`/Engine/EditorBlueprintResources/StandardMacros.IsValid` (`self.SandSystemRef`)
    (:`Is Not Valid`
      (bind _returnvalue (`NiagaraFunctionLibrary.SpawnSystemAttached` "/Game/Misc/Niagara/NS_Sand.NS_Sand" (`self.RootComponent`) "None" (`KismetMathLibrary.MakeVector` 0.0 0.0 (- (.z HitLocation) (.z (`self.K2_GetActorLocation`)))) (struct) "KeepRelativeOffset" true))
      (bind _output_get (set `self.SandSystemRef` _returnvalue))
      (`VisualLoggerKismetLibrary.LogText` null "System Spawned" "VisLogBP" true))))

(fn `UserConstructionScript`)