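; BP_PlayerShip is the player ship Blueprint, whose visible logic handles only the pause menu.
; On BeginPlay it creates a PauseScreen1 widget, adds it to the viewport hidden and makes it focusable.
; The Pause input reveals the widget, pauses the game, switches to UI-only input focused on it, and moves the mouse just below screen center.
; No unpause logic appears here, and the construction script is empty.
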(event `self.ReceiveBeginPlay`
  (bind _returnvalue (`|CreateWidget` "/Game/Blueprints/UI/PauseScreen1.PauseScreen1_C"))
  (`UserWidget.AddToViewport` _returnvalue 0)
  (`Widget.SetVisibility` _returnvalue "Hidden")
  (set `UserWidget.bIsFocusable` true _returnvalue))

(event `InputAction|Pause`
  (params (Key :type "Key Structure"))
  (bind _returnvalue (`GameplayStatics.GetPlayerController` 0))
  (bind (_sizex _sizey) (`PlayerController.GetViewportSize` _returnvalue))
  (:`Pressed`
    (`Widget.SetVisibility` (stale `self.ReceiveBeginPlay` _returnvalue) "Visible")
    (`GameplayStatics.SetGamePaused` true)
    (`WidgetBlueprintLibrary.SetInputMode_UIOnlyEx` _returnvalue (stale `self.ReceiveBeginPlay` _returnvalue))
    (`PlayerController.SetMouseLocation` _returnvalue (/ _sizex 2) (+ (/ _sizey 2) 100))))

(fn `UserConstructionScript`)